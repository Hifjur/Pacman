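; BP_Enemy is a Pac-Man-style chasing enemy character that either kills the player on contact or is killed by a powered-up one.
; It sets its walk speed on BeginPlay and uses PawnSensing to start an AIMoveTo toward the player when it sees a pawn.
; On a capsule hit with BP_ThirdPersonCharacter, it reads power-up state from the player's mesh material, destroying itself for MI_PacmanpoweredUP and the player otherwise.
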(event `self.ReceiveBeginPlay`
  (set `CharacterMovementComponent.MaxWalkSpeed` 450.0 (`self.CharacterMovement`)))

(event `self.PawnSensing.OnSeePawn`
  (params (Pawn :type "Pawn Object Reference"))
  (`|AIMoveTo` self (0.0 0.0 0.0) (`GameplayStatics.GetPlayerCharacter` 0)))

(event `self.CapsuleComponent.OnComponentHit`
  (params (HitComponent :type "PrimitiveComponent Object Reference") (OtherActor :type "Actor Object Reference") (OtherComp :type "PrimitiveComponent Object Reference") (NormalImpulse :type "Vector Structure") (Hit :type "HitResult Structure (by ref)"))
  (bind _asbp_third_person_character (cast `/Game/ThirdPerson/Blueprints/BP_ThirdPersonCharacter` OtherActor))
  (if (== (`PrimitiveComponent.GetMaterial` (`Character.Mesh` _asbp_third_person_character) 0) "/Game/Materials/MI_PacmanpoweredUP.MI_PacmanpoweredUP")
    (`self.K2_DestroyActor`)
    (else
      (`self.K2_DestroyActor` _asbp_third_person_character))))

(fn `UserConstructionScript`)