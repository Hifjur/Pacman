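; Player controller for the Pac-Man pawn that turns directional input into continuous movement.
; On possess it casts the pawn to BP_PacmanPlayer and caches the reference.
; The four input actions only write a direction to the pawn's MoveState, with no release handling.
; Tick reads that state and calls the matching move function on the pawn, so the last pressed direction keeps applying.
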(event `self.ReceivePossess`
  (params (PossessedPawn :type "Pawn Object Reference"))
  (bind _asbp_pacman_player (cast `/Game/Blueprints/BP_PacmanPlayer` PossessedPawn))
  (set `self.As BP Pacman Player` _asbp_pacman_player))

(event `self.ReceiveTick`
  (params (DeltaSeconds :type "Float (single-precision)"))
  (if (== 1 (stale `InputAction|MoveRight` _output_get))
    (`/Game/Blueprints/BP_PacmanPlayer.MoveRight` (`self.As BP Pacman Player`))
    (elif (== (stale `InputAction|MoveLeft` _output_get) 2)
      (`/Game/Blueprints/BP_PacmanPlayer.MoveLeft` (`self.As BP Pacman Player`))
      (elif (== (stale `InputAction|MoveUp` _output_get) 3)
        (`/Game/Blueprints/BP_PacmanPlayer.MoveUP` (`self.As BP Pacman Player`))
        (elif (== (stale `InputAction|MoveDown` _output_get) 4)
          (`/Game/Blueprints/BP_PacmanPlayer.MoveDown` (`self.As BP Pacman Player`)))))))

(event `InputAction|MoveRight`
  (params (Key :type "Key Structure"))
  (:`Pressed`
    (bind _output_get (set `/Game/Blueprints/BP_PacmanPlayer.MoveState` 1 (`self.As BP Pacman Player`)))))

(event `InputAction|MoveLeft`
  (params (Key :type "Key Structure"))
  (:`Pressed`
    (bind _output_get (set `/Game/Blueprints/BP_PacmanPlayer.MoveState` 2 (`self.As BP Pacman Player`)))))

(event `InputAction|MoveUp`
  (params (Key :type "Key Structure"))
  (:`Pressed`
    (bind _output_get (set `/Game/Blueprints/BP_PacmanPlayer.MoveState` 3 (`self.As BP Pacman Player`)))))

(event `InputAction|MoveDown`
  (params (Key :type "Key Structure"))
  (:`Pressed`
    (bind _output_get (set `/Game/Blueprints/BP_PacmanPlayer.MoveState` 4 (`self.As BP Pacman Player`)))))

(fn `UserConstructionScript`)