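; Pac-Man player Blueprint that provides movement steps for the character along the world X and Y axes.
; Four directional events each nudge the skeletal mesh by a fixed world-space offset, without sweeping for collisions.
; Box overlap or hit events reset MoveState to zero; this graph neither reads that variable nor calls the movement events.
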(event `MoveRight`
  (bind _skeletalmesh (`self.SkeletalMesh`))
  (`SceneComponent.K2_SetWorldLocation` _skeletalmesh (+ (`SceneComponent.K2_GetComponentLocation` _skeletalmesh) (0.0 10.0 0.0)) false false))

(event `MoveLeft`
  (bind _skeletalmesh (`self.SkeletalMesh`))
  (`SceneComponent.K2_SetWorldLocation` _skeletalmesh (+ (`SceneComponent.K2_GetComponentLocation` _skeletalmesh) (0.0 -10.0 0.0)) false false))

(event `MoveUP`
  (bind _skeletalmesh (`self.SkeletalMesh`))
  (`SceneComponent.K2_SetWorldLocation` _skeletalmesh (+ (`SceneComponent.K2_GetComponentLocation` _skeletalmesh) (10.0 0.0 0.0)) false false))

(event `MoveDown`
  (bind _skeletalmesh (`self.SkeletalMesh`))
  (`SceneComponent.K2_SetWorldLocation` _skeletalmesh (+ (`SceneComponent.K2_GetComponentLocation` _skeletalmesh) (-10.0 0.0 0.0)) false false))

(event `self.Box.OnComponentBeginOverlap`
  (params (OverlappedComponent :type "PrimitiveComponent Object Reference") (OtherActor :type "Actor Object Reference") (OtherComp :type "PrimitiveComponent Object Reference") (OtherBodyIndex :type Integer) (bFromSweep :type Boolean) (SweepResult :type "HitResult Structure (by ref)"))
  (set `self.MoveState` 0 :!label _label))

(event `self.Box.OnComponentHit`
  (params (HitComponent :type "PrimitiveComponent Object Reference") (OtherActor :type "Actor Object Reference") (OtherComp :type "PrimitiveComponent Object Reference") (NormalImpulse :type "Vector Structure") (Hit :type "HitResult Structure (by ref)"))
  (goto _label))

(fn `UserConstructionScript`)